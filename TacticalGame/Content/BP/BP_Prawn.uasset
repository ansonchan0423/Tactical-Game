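; BP_Prawn is a camera rig with a spring arm, moved and zoomed by player axis input.
; Forward/backward and left/right inputs shift a desired location along world X and Y, while zoom input adjusts a clamped desired arm length.
; Tick interpolates the actor location and spring arm length toward those targets, smoothing both pan and zoom.
; BeginPlay only assigns both target variables to themselves, so they start at their default values.
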(event `self.ReceiveBeginPlay`
  (set `self.Zoom_desired` (`self.Zoom_desired`))
  (set `self.Location_desired` (`self.Location_desired`)))

(event `InputAxis|InputAxis_Zoom`
  (params (AxisValue :type "Float (single-precision)"))
  (set `self.Zoom_desired` (`KismetMathLibrary.FClamp` (+ (* AxisValue 100.0) (`self.Zoom_desired`)) 100.0 5000.0)))

(event `self.ReceiveTick`
  (params (DeltaSeconds :type "Float (single-precision)"))
  (bind _springarm (`self.SpringArm`))
  (set `SpringArmComponent.TargetArmLength` (`KismetMathLibrary.FInterpTo` (`SpringArmComponent.TargetArmLength` _springarm) (`self.Zoom_desired`) DeltaSeconds 2.0) _springarm)
  (`self.K2_SetActorLocation` (`KismetMathLibrary.VInterpTo` (`self.K2_GetActorLocation`) (`self.Location_desired`) DeltaSeconds 20.0)))

(event `InputAxis|InputAxis_Forward_Backward`
  (params (AxisValue :type "Float (single-precision)"))
  (set `self.Location_desired` (+ (`self.Location_desired`) (`KismetMathLibrary.MakeVector` (* AxisValue 20.0)))))

(event `InputAxis|InputAxis_Left_Right`
  (params (AxisValue :type "Float (single-precision)"))
  (set `self.Location_desired` (+ (`self.Location_desired`) (`KismetMathLibrary.MakeVector` 0.0 (* AxisValue 20.0)))))

(fn `UserConstructionScript`)